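; GA_Skill1 is a Gameplay Ability for the first skill slot that plays a standing one-handed magic attack montage, with no damage or effects yet.
; A ValidateAbility macro checks the avatar character and commits the ability, cancelling or ending it on failure.
; On commit it prints a debug string and plays the montage from its Cast section.
; Only montage completion ends the ability, as interrupted and cancelled outputs are unhandled.
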(event `self.K2_ActivateAbility`
  (`self.ValidateAbility`
    (:`OnCommit`
      (`KismetSystemLibrary.PrintString` "Skill 1")
      (`AbilityTask_PlayMontageAndWait.CreatePlayMontageAndWaitProxy` "None" "/Game/Mixamo/MagicSpellPack/Animations/S_Standing_1H_Magic_Attack_01_Montage.S_Standing_1H_Magic_Attack_01_Montage" 1.0 "Cast"
        (:`OnCompleted`
          (`self.K2_EndAbility`))))
    (:`OnCancel`
      (`self.K2_EndAbility`))))