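; GA_Jump is a gameplay ability that makes the avatar character jump.
; CanActivateAbility allows it only while a valid avatar's movement component reports moving on ground.
; On activation it commits, starts a WaitInputRelease task, then calls Jump and immediately ends the ability.
; StopJumping is wired to the release callback, though the ability has already ended by then; a failed commit cancels it.
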(event `self.K2_ActivateAbility`
  (bind _returnvalue (`self.GetAvatarCharacter`))
  (`/Engine/EditorBlueprintResources/StandardMacros.IsValid` _returnvalue
    (:`Is Valid`
      (bind _returnvalue_2 (`self.K2_CommitAbility`))
      (if _returnvalue_2
        (`AbilityTask_WaitInputRelease.WaitInputRelease` true
          (:`then`
            (`Character.Jump` _returnvalue)
            (`self.K2_EndAbility`))
          (:`OnRelease`
            (`Character.StopJumping` _returnvalue)))
        (else
          (`self.K2_CancelAbility`))))
    (:`Is Not Valid`
      (`self.K2_EndAbility`))))

(fn `K2_CanActivateAbility`
  (params (ActorInfo :type "GameplayAbilityActorInfo Structure") (Handle :type "GameplayAbilitySpecHandle Structure"))
  (returns (RelevantTags :type "GameplayTagContainer Structure") (ReturnValue :type Boolean))
  (bind _returnvalue (`self.GetAvatarCharacter`))
  (`/Engine/EditorBlueprintResources/StandardMacros.IsValid` _returnvalue
    (:`Is Valid`
      (if (`NavMovementComponent.IsMovingOnGround` (`Character.CharacterMovement` _returnvalue))
        (return (struct) true)
        (else
          _)))
    (:`Is Not Valid`
      _))
  (return (struct) false))