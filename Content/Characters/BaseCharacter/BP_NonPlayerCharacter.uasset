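; BP_NonPlayerCharacter is a bot character that carries a nameplate and periodically jumps through the Gameplay Ability System.
; After ability system initialization, a looping timer tries to activate GA_Jump on its ability system component.
; It also creates a WBP_NamePlate labeled "Manny Bot" and binds it to that component, retrying each tick until this succeeds before assigning it to the Nameplate component.
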(event `self.PostInitializeAbilitySystem`
  (`KismetSystemLibrary.K2_SetTimerDelegate` (delegate `Jump GA`) 3.0 true true)
  (bind _returnvalue (`|CreateWidget` "/Game/UI/WBP_NamePlate.WBP_NamePlate_C" null "Manny Bot"))
  (bind _output_get (set `self.NamePlate Widget` _returnvalue))
  (`/Engine/EditorBlueprintResources/StandardMacros.IsValid` _output_get
    (:`Is Valid`
      (bind _returnvalue_2 (`AbilitySystemWidget.InitializeAbilitySystemWidget` (`self.NamePlate Widget`) (`AbilitySystemBlueprintLibrary.GetAbilitySystemComponent` self) :!label _label))
      (if _returnvalue_2
        (`WidgetComponent.SetWidget` (`self.Nameplate`) (`self.NamePlate Widget`))
        (else
          (`KismetSystemLibrary.DelayUntilNextTick`)
          (goto _label))))))

(event `Jump GA`
  (`AbilitySystemComponent.TryActivateAbilityByClass` (`AbilitySystemBlueprintLibrary.GetAbilitySystemComponent` self) "/Game/AbilitySystem/GameplayAbilities/GA_Jump.GA_Jump_C" true))

(fn `UserConstructionScript`)