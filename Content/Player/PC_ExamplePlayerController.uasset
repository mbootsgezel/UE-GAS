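; Example player controller that creates the in-game UI for the local player.
; On BeginPlay it creates WBP_InGameUI and passes the controlled pawn's Ability System Component to the widget's initialization.
; If initialization fails, it retries each tick until it succeeds, and only then adds the widget to the viewport.
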(event `self.ReceiveBeginPlay`
  (if (`self.IsLocalPlayerController`)
    (bind _returnvalue (`|CreateWidget` "/Game/UI/WBP_InGameUI.WBP_InGameUI_C" self))
    (bind _output_get (set `self.InGameUI` _returnvalue))
    (`/Engine/EditorBlueprintResources/StandardMacros.IsValid` _output_get
      (:`Is Valid`
        (bind _returnvalue_2 (`AbilitySystemWidget.InitializeAbilitySystemWidget` (`self.InGameUI`) (`AbilitySystemBlueprintLibrary.GetAbilitySystemComponent` (`self.K2_GetPawn`)) :!label _label))
        (if _returnvalue_2
          (`UserWidget.AddToViewport` (`self.InGameUI`) 0)
          (else
            (`KismetSystemLibrary.DelayUntilNextTick`)
            (goto _label)))))))

(fn `UserConstructionScript`)